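; Survival game mode Blueprint that announces each incoming enemy wave with an on-screen countdown.
; On BeginPlay it binds to its state-changed dispatcher and reacts only to the Wait Spawn New Wave state.
; That state creates a WBP_WaveTextWithCountDown widget, sets its text from the current wave count, and starts its countdown using the spawn wait time.
; Wave spawning and state transitions are not handled in these graphs.
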(event Custom|OnSurvialGameModeStateChanged_事件
  (params (CurrentState :type EWarriorSurvialGameModeState%20Enum :default "WaitSpawnNewWave"))
  (switch Utilities|FlowControl|Switch|SwitchonEWarriorSurvialGameModeState CurrentState
    (:WaitSpawnNewWave
      (CallFunction|CreateNewWaveWidgetwithCountDown (Utilities|Text|FormatText "Wave {CurrentWave} Coming In" (Variables|Default|GetCurrentWaveCount)) (Variables|Default|GetSpawnNewWaveWaitTime)))))

(event EventBeginPlay
  (EventDispatchers|AssignOnSurvialGameModeStateChanged (delegate Custom|OnSurvialGameModeStateChanged_事件)))

(event EventTick
  (params (DeltaSeconds :type Float%20%28single-precision%29)))

(fn ConstructionScript)

(fn CreateNewWaveWidgetwithCountDown
  (params (InTextToDisplay :type Text) (InTotalCountDownTime :type Float%20%28double-precision%29))
  (bind _returnvalue (UserInterface|CreateWidget "/Game/Widget/GameModeWidgets/WBP_WaveTextWithCountDown.WBP_WaveTextWithCountDown_C"))
  (UserInterface|Viewport|AddtoViewport _returnvalue 0)
  (Rendering|Components|TextRender|SetText (Variables|/Game/Widget/GameModeWidgets/WBP_WaveTextWithCountDown.WBP_WaveTextWithCountDown_C|GetTextBlock_CountDownNum _returnvalue) InTextToDisplay)
  (Default|StartCountDown _returnvalue InTotalCountDownTime))